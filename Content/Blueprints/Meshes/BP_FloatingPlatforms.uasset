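; Floating platform actor, labelled a ramming platform, that endlessly travels up and down between two fixed world heights from BeginPlay.
; It steps its Z offset in looping short Delays instead of Tick or a Timeline, pausing at each end.
; IsMoving and IsActive flags gate the turnarounds.
; The bad-coding graph holds an earlier-looking, never-run variant that derives its step from a counter.
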(event EventBeginPlay
  (bind _returnvalue (Transformation|GetActorLocation))
  ;[1 1 1] Ramming Platform
  (|CallParentFunction)
  (if (not (and (Variables|Default|GetisActive) (Variables|Default|GetisMoving))) :!label _label
    (Math|Float|CompareFloat (.z _returnvalue) 3e+02 :!label _label_2
      (:>
        _)
      (:==
        _)
      (:<
        (Variables|Default|SetisMoving true)
        (Transformation|AddActorLocalOffset (Math|Vector|MakeVector 0.0 0.0 2.0) false false)
        (Utilities|FlowControl|Delay 0.01)
        (goto _label_2)))
    (Utilities|FlowControl|Sequence
      (:then_0
        (Variables|Default|SetisMoving false))
      (:then_1
        (Variables|Default|SetisActive true))
      (:then_2
        (Utilities|FlowControl|Delay 1.5)
        (if (not (Variables|Default|GetisMoving))
          (Math|Float|CompareFloat (.z _returnvalue) 1e+02 :!label _label_3
            (:>
              (Variables|Default|SetisMoving true)
              (Transformation|AddActorLocalOffset (Math|Vector|MakeVector 0.0 0.0 -2.0) false false)
              (Utilities|FlowControl|Delay 0.01)
              (goto _label_3))
            (:==
              _)
            (:<
              _))
          (Utilities|FlowControl|Sequence
            (:then_0
              (Variables|Default|SetisMoving false))
            (:then_1
              (Variables|Default|SetisActive false))
            (:then_2
              (Utilities|FlowControl|Delay 1.5)
              (goto _label))))))))

(fn ConstructionScript
  (|CallParentFunction))