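; Door actor that swings open when something overlaps its Box trigger and closes when the overlap ends.
; Delay loops rotate the whole actor one degree per step, using counter I to stop at 90 or 0.
; The Anim flag blocks both events during movement, so an overlap change mid-swing is dropped rather than queued.
; The overlapping actor is not filtered.
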(event OnComponentBeginOverlap(Box)
  (params (OverlappedComponent :type Primitive%20Component%20Object%20Reference) (OtherActor :type Actor%20Object%20Reference) (OtherComp :type Primitive%20Component%20Object%20Reference) (OtherBodyIndex :type Integer) (bFromSweep :type Boolean) (SweepResult :type Hit%20Result%20Structure%20%28by%20ref%29))
  (bind _i (Variables|Default|Geti))
  (if (not (Variables|Default|Getanim?))
    (Math|Integer|CompareInt _i 90 :!label _label
      (:>
        _)
      (:==
        _)
      (:<
        (Math|Integer|IncrementInt _i
          (:%20%20
            (Variables|Default|Setanim? true)
            (Transformation|AddActorLocalRotation "0,1.000000, 0" false false)
            (Utilities|FlowControl|Delay 0.01)
            (goto _label)))))
    (Variables|Default|Setanim? false)))

(event OnComponentEndOverlap(Box)
  (params (OverlappedComponent :type Primitive%20Component%20Object%20Reference) (OtherActor :type Actor%20Object%20Reference) (OtherComp :type Primitive%20Component%20Object%20Reference) (OtherBodyIndex :type Integer))
  (bind _i (Variables|Default|Geti))
  (if (not (Variables|Default|Getanim?))
    (Math|Integer|CompareInt _i :!label _label
      (:>
        (Math|Integer|DecrementInt _i
          (:%20%20
            (Variables|Default|Setanim? true)
            (Transformation|AddActorLocalRotation "0,-1.000000, 0" false false)
            (Utilities|FlowControl|Delay 0.01)
            (goto _label))))
      (:==
        _)
      (:<
        _))
    (Variables|Default|Setanim? false)))

(event EventBeginPlay)

(fn ConstructionScript)