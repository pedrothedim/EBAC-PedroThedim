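; BP_collectibles is a collectible actor that spins, floats and reacts when the player character touches it.
; Two endless Delay loops from BeginPlay animate it: one yaws the actor, the other offsets the mesh height along the looping FloatingFx curve.
; Sphere overlap with BP_pCharacter stores the player, calls the empty Collect event as a hook, then destroys the actor if IsCollectible is set.
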(event OnComponentBeginOverlap(Sphere)
  (params (OverlappedComponent :type Primitive%20Component%20Object%20Reference) (OtherActor :type Actor%20Object%20Reference) (OtherComp :type Primitive%20Component%20Object%20Reference) (OtherBodyIndex :type Integer) (bFromSweep :type Boolean) (SweepResult :type Hit%20Result%20Structure%20%28by%20ref%29))
  (bind _asbp_p_character (Utilities|Casting|CastToBP_pCharacter OtherActor))
  (Variables|Default|SetPlayer _asbp_p_character)
  (CallFunction|Collect)
  (if (Variables|Default|GetisCollectible)
    (Actor|DestroyActor)))

(event Custom|Collect)

(event EventBeginPlay
  (bind _staticmesh (Variables|Default|GetStaticMesh))
  (Utilities|FlowControl|Sequence
    (:then_0
      (Transformation|AddActorLocalRotation "0.000000,1.000000, 0" false false :!label _label)
      (Utilities|FlowControl|Delay 0.01)
      (goto _label))
    (:then_1
      (Variables|Default|SetinitialLocation (Variables|/Script/Engine.SceneComponent|GetRelativeLocation _staticmesh))
      (Transformation|SetRelativeLocation _staticmesh (Math|Vector|MakeVector (.x (Variables|Default|GetinitialLocation)) (.y (Variables|Default|GetinitialLocation)) (+ (.z (Variables|Default|GetinitialLocation)) (Math|Curves|GetFloatValue (Variables|Default|GetfloatingFx) (Variables|Default|GetIn%20Time)))) false false :!label _label_2)
      (bind _output_get (Variables|Default|SetIn%20Time (+ (Variables|Default|GetIn%20Time) 0.05)))
      (if (> _output_get 5.0)
        (Variables|Default|SetIn%20Time 0.0))
      (Utilities|FlowControl|Delay 0.01)
      (goto _label_2))))

(fn ConstructionScript)