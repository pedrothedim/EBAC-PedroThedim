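; BP_MedKits is a medkit pickup that heals the player when collected.
; Its Collect event calls ChangeHealth on the Player, then sets the Player's Heal to a fixed amount after that call.
; BeginPlay and the construction script only call their parents.
; An unused backup graph holds older local logic that caps health at full, toggles IsCollectible and prints health or a delay-throttled full-health message.
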(event EventBeginPlay
  (|CallParentFunction))

(event EventCollect
  (bind _player (Variables|Default|GetPlayer))
  (Default|ChangeHealth _player true)
  (Variables|/Game/0_EBAC-Modulos/Modulo5/BP_pCharacter.BP_pCharacter_C|SetHeal _player 25.0))

(fn ConstructionScript
  (|CallParentFunction))