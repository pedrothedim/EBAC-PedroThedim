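; BP_CurveEx is a learning Blueprint that animates a static mesh vertically using a float curve, as a floating effect.
; On BeginPlay it stores the mesh's initial relative location, then offsets Z by the FloatingFx curve value sampled at InTime.
; A self-looping Delay, rather than Tick or a Timeline, advances InTime in fixed steps and resets it to zero past a limit.
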(event EventBeginPlay
  (bind _staticmesh (Variables|Default|GetStaticMesh))
  (Variables|Default|SetinitialLocation (Variables|/Script/Engine.SceneComponent|GetRelativeLocation _staticmesh))
  (Transformation|SetRelativeLocation _staticmesh (Math|Vector|MakeVector (.x (Variables|Default|GetinitialLocation)) (.y (Variables|Default|GetinitialLocation)) (+ (.z (Variables|Default|GetinitialLocation)) (Math|Curves|GetFloatValue (Variables|Default|GetfloatingFx) (Variables|Default|GetIn%20Time)))) false false :!label _label)
  (bind _output_get (Variables|Default|SetIn%20Time (+ (Variables|Default|GetIn%20Time) 0.05)))
  (if (> _output_get 5.0)
    (Variables|Default|SetIn%20Time 0.0))
  (Utilities|FlowControl|Delay 0.01)
  (goto _label))

(fn ConstructionScript)