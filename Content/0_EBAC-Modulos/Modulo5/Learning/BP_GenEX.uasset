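; BP_GenEX is a learning Blueprint with unconnected experiments for setting Health from a character Class (Warrior, Ranger, Sorcerer or Scout).
; One approach reverse-looks up the Classes map, looping over its values to find the Class and taking the key at that index as Health.
; Another uses a Select node to pick a fixed Health per class.
; None of this logic runs, as BeginPlay and the construction script are empty.
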(event EventBeginPlay)

(fn ConstructionScript)