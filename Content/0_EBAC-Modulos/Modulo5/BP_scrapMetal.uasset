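; BP_scrapMetal is a scrap metal pickup that adds to the player's scrap count when collected.
; Its Collect event increments Scraps on the Player reference, then prints the new total as a formatted "Sucata" debug message.
; The Blueprint itself holds no overlap detection or destroy logic, and its BeginPlay and construction script add no behavior.
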(event EventBeginPlay
  (|CallParentFunction) ; This node is disabled and will not be called.\nDrag off pins to build functionality.
)

(event EventCollect
  (bind _player (Variables|Default|GetPlayer))
  (bind _result (Math|Integer|IncrementInt (Variables|/Game/0_EBAC-Modulos/Modulo5/BP_pCharacter.BP_pCharacter_C|Getscraps _player))
    (:%20%20
      (bind _output_get (Variables|/Game/0_EBAC-Modulos/Modulo5/BP_pCharacter.BP_pCharacter_C|Setscraps _player _result))
      (Development|PrintString (Utilities|String|ToString(Text) (Utilities|Text|FormatText "Sucata: {scraps}" _output_get))))))

(fn ConstructionScript
  (|CallParentFunction))