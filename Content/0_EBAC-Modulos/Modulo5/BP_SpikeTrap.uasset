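; BP_SpikeTrap is a spike trap that affects a BP_pCharacter entering its Box collision.
; On overlap it calls the character's ChangeHealth with false, then sets that character's Damage variable, so the assignment follows the health change.
; A disconnected backup graph holds an older direct health subtraction with a warning print and a delay-based hit cooldown, none of which runs.
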(event OnComponentBeginOverlap(Box)
  (params (OverlappedComponent :type Primitive%20Component%20Object%20Reference) (OtherActor :type Actor%20Object%20Reference) (OtherComp :type Primitive%20Component%20Object%20Reference) (OtherBodyIndex :type Integer) (bFromSweep :type Boolean) (SweepResult :type Hit%20Result%20Structure%20%28by%20ref%29))
  (bind _asbp_p_character (Utilities|Casting|CastToBP_pCharacter OtherActor))
  (Default|ChangeHealth _asbp_p_character false)
  (Variables|/Game/0_EBAC-Modulos/Modulo5/BP_pCharacter.BP_pCharacter_C|SetDamage _asbp_p_character 5e+01))

(fn ConstructionScript)