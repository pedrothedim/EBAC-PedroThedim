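; BP_Donut is a spinning pickup that disappears when touched and respawns in place.
; A looping short Delay from BeginPlay rotates the Donut component in small fixed steps, without using Tick.
; Any overlap on the Capsule while visible hides the actor, spawns an explosion particle at its location, and unhides it after a few seconds.
; The hidden flag doubles as the guard against repeat triggers, and nothing is awarded to the overlapping actor.
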(event OnComponentBeginOverlap(Capsule)
  (params (OverlappedComponent :type Primitive%20Component%20Object%20Reference) (OtherActor :type Actor%20Object%20Reference) (OtherComp :type Primitive%20Component%20Object%20Reference) (OtherBodyIndex :type Integer) (bFromSweep :type Boolean) (SweepResult :type Hit%20Result%20Structure%20%28by%20ref%29))
  ;[1 1 1] Collect / Respawn
  (if (not (Variables|Rendering|GetbHidden))
    (Rendering|SetActorHiddenInGame true)
    (Utilities|FlowControl|Sequence
      (:then_0
        (Effects|SpawnEmitteratLocation "/Game/StarterContent/Particles/P_Explosion.P_Explosion" (Transformation|GetActorLocation)))
      (:then_1
        (Utilities|FlowControl|Delay 3.0)
        (Rendering|SetActorHiddenInGame false)))))

(event EventBeginPlay
  ;[1 1 1] Rotation
  (Transformation|AddLocalRotation (Variables|Default|GetDonut) "0,1.000000, 0" false false :!label _label)
  (Utilities|FlowControl|Delay 0.01)
  (goto _label))

(fn ConstructionScript)