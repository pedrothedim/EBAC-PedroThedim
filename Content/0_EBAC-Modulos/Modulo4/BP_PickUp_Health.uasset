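; BP_PickUp_Health is a health pickup that adds its HealthPool value to the player's Health.
; Its PickUpEffect event spawns an explosion particle at the pickup's location, applies the health increase without any clamp, then prints the new Health.
; The construction script only calls its parent, and this graph contains no overlap detection or destroy logic.
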(event EventPickUpEffect
  (bind _player (Variables|Default|Getplayer))
  (Effects|SpawnEmitteratLocation "/Game/StarterContent/Particles/P_Explosion.P_Explosion" (Transformation|GetActorLocation))
  (bind _output_get (Variables|/Game/ThirdPerson/Blueprints/BP_ThirdPersonCharacter_TEST.BP_ThirdPersonCharacter_TEST_C|Sethealth _player (+ (Variables|/Game/ThirdPerson/Blueprints/BP_ThirdPersonCharacter_TEST.BP_ThirdPersonCharacter_TEST_C|Gethealth _player) (Variables|Default|GethealthPool))))
  (Development|PrintString (Utilities|String|ToString(Float) _output_get)))

(fn ConstructionScript
  (|CallParentFunction))