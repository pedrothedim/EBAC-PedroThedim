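; Coin pickup that adds one to the player's Currency when its pickup effect fires.
; It extends a parent Blueprint, overriding PickUpEffect to increment the counter on the Player reference and print the result to screen.
; From BeginPlay, a looping short Delay continually applies a small local rotation to the static mesh, spinning the coin in fixed steps without Tick or frame-time scaling.
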(event EventBeginPlay
  (|CallParentFunction)
  (Transformation|AddLocalRotation (Variables|Default|GetStaticMesh) "0,0.500000, 0" false false :!label _label)
  (Utilities|FlowControl|Delay 0.01)
  (goto _label))

(event EventPickUpEffect
  (bind _result (Math|Integer|IncrementInt (Variables|/Game/ThirdPerson/Blueprints/BP_ThirdPersonCharacter_TEST.BP_ThirdPersonCharacter_TEST_C|GetCurrency (Variables|Default|Getplayer)))
    (:%20%20
      (Development|PrintString (Utilities|String|ToString(Integer) _result)))))

(fn ConstructionScript
  (|CallParentFunction))