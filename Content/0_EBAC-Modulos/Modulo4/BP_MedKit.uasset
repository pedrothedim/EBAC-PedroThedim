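; BP_MedKit is a health pickup that heals the player character when its sphere collision registers an overlap.
; On overlap it casts player 0's character to BP_ThirdPersonCharacter_TEST without checking which actor overlapped, then adds Heal to Health, capped at its own MaxHealth.
; It prints the resulting health and stays in the level, with no destroy or single-use logic.
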(event OnComponentBeginOverlap(Sphere)
  (params (OverlappedComponent :type Primitive%20Component%20Object%20Reference) (OtherActor :type Actor%20Object%20Reference) (OtherComp :type Primitive%20Component%20Object%20Reference) (OtherBodyIndex :type Integer) (bFromSweep :type Boolean) (SweepResult :type Hit%20Result%20Structure%20%28by%20ref%29))
  (bind _maxhealth (Variables|Default|GetmaxHealth))
  (bind _asbp_third_person_character_test (Utilities|Casting|CastToBP_ThirdPersonCharacter_TEST (Game|GetPlayerCharacter 0)))
  (Math|Float|CompareFloat (+ (Variables|Default|Getheal) (Variables|/Game/ThirdPerson/Blueprints/BP_ThirdPersonCharacter_TEST.BP_ThirdPersonCharacter_TEST_C|Gethealth _asbp_third_person_character_test)) _maxhealth
    (:>
      (bind _output_get (Variables|/Game/ThirdPerson/Blueprints/BP_ThirdPersonCharacter_TEST.BP_ThirdPersonCharacter_TEST_C|Sethealth _asbp_third_person_character_test _maxhealth :!label _label))
      (Development|PrintString (Utilities|String|ToString(Float) _output_get)))
    (:==
      (goto _label))
    (:<
      (bind _output_get_2 (Variables|/Game/ThirdPerson/Blueprints/BP_ThirdPersonCharacter_TEST.BP_ThirdPersonCharacter_TEST_C|Sethealth _asbp_third_person_character_test (+ (Variables|Default|Getheal) (Variables|/Game/ThirdPerson/Blueprints/BP_ThirdPersonCharacter_TEST.BP_ThirdPersonCharacter_TEST_C|Gethealth _asbp_third_person_character_test))))
      (Development|PrintString (Utilities|String|ToString(Float) _output_get_2)))))

(event EventBeginPlay
  (|CallParentFunction))

(fn ConstructionScript
  (|CallParentFunction))